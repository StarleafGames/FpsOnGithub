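; Timed ammo pickup that refills the primary weapon of a living BP_CharacterMaster that overlaps it.
; Overlap tops that weapon's AmmoBag up to a hard-coded minimum, plays the health pickup cue, then destroys the actor after a short delay, even if no ammo was needed.
; BeginPlay sets a lifespan so unclaimed packs expire.
; Heal and pickup-sound events are empty stubs, and an older active-item refill is disabled.
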(event Custom|SV_RestoreHealth
  (params (Object :type Object%20Object%20Reference))
  ;[0 0 0] Heal
)

(event Custom|OC_PickupSound)

(event EventBeginPlay
  ;[0 0 0] Beginplay
  (Variables|Default|GetAmmoPack
    (:then
      (Actor|SetLifeSpan 15.0))
    (:else)))

(event Collision|EventActorBeginOverlap
  (params (OtherActor :type Actor%20Object%20Reference))
  ;[0 0 0] Actor overlap
  (bind _asbp_character_master (Utilities|Casting|CastToBP_CharacterMaster OtherActor))
  (bind _output_get (Variables|Default|SetAs%20BP%20Character%20Master _asbp_character_master))
  (if (not (Variables|/Game/TrueFPS/Characters/BP_CharacterMaster.BP_CharacterMaster_C|GetDead? _output_get))
    (Utilities|FlowControl|Sequence
      (:then_0
        (bind _primary (Variables|/Game/TrueFPS/Characters/BP_CharacterMaster.BP_CharacterMaster_C|GetPrimary (Variables|Default|GetAs%20BP%20Character%20Master))
          (:then
            (if (< (Variables|/Game/TrueFPS/Items/Weapons/BP_WeaponMaster.BP_WeaponMaster_C|GetAmmoBag _primary) 120)
              (Variables|/Game/TrueFPS/Items/Weapons/BP_WeaponMaster.BP_WeaponMaster_C|SetAmmoBag _primary 120)))
          (:else)))
      (:then_1
        (Audio|PlaySoundatLocation "/Game/TrueFPS/Effects/Sounds/Pickups/SCue_Pickup_Health.SCue_Pickup_Health" (Transformation|GetActorLocation) "0, 0, 0" 0.5 1.0 0.0 "/Game/TrueFPS/Characters/Audio/AT_Player.AT_Player" 0 OtherActor 0))
      (:then_2
        (Utilities|FlowControl|Delay 0.3)
        (Actor|DestroyActor)))))

(fn ConstructionScript)

(fn OnRepHeal)