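; Spawner actor that keeps an ammo pickup available at its own location in the level.
; On BeginPlay it spawns an Ammo_Pickup with a short lifespan and starts a looping timer.
; Each timer tick spawns a replacement only if the stored pack reference is no longer valid.
; Only the initial pack is given a lifespan; respawned packs get none set here.
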(event Custom|Respawner
  ;[0 0 0] Respawner
  (Variables|Default|GetAmmoPack
    (:then)
    (:else
      (bind _returnvalue (Game|SpawnActorfromClass "/Game/Blueprints/Pick-Ups/Ammo_Pickup.Ammo_Pickup_C" (Transformation|GetActorTransform) "AdjustIfPossibleButAlwaysSpawn" 0 0))
      (Variables|Default|SetAmmoPack _returnvalue))))

(event EventBeginPlay
  ;[0 0 0] Beginplay
  ;[0 0 0] Initial Pack Spawn
  (bind _returnvalue (Game|SpawnActorfromClass "/Game/Blueprints/Pick-Ups/Ammo_Pickup.Ammo_Pickup_C" (Transformation|GetActorTransform) "AdjustIfPossibleButAlwaysSpawn" 0 0))
  (bind _output_get (Variables|Default|SetAmmoPack _returnvalue))
  (Actor|SetLifeSpan _output_get 1e+01)
  ;[0 0 0] Respawn Timer
  (bind _returnvalue_2 (Utilities|Time|SetTimerbyEvent (delegate Custom|Respawner) 1e+01 true))
  (Variables|Default|SetRespawnerTimer _returnvalue_2))

(event Collision|EventActorBeginOverlap
  (params (OtherActor :type Actor%20Object%20Reference)))

(fn ConstructionScript)