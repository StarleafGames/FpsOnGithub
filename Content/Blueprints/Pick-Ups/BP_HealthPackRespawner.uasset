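; Health pack respawner actor that spawns a BP_HealthPickup at its own transform, with a text-render countdown.
; BeginPlay sets the game mode as owner and, if Timer is zero, resets it and replaces the pack.
; Clients_Timer decrements and displays Timer through RespawnTime, then calls the empty ServerRespawn.
; The looping timer setup and Clients_Timer call are disconnected, so nothing here drives repeat respawns.
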(event Custom|SvrReplicate
  ;[0 0.07632 1] Replicate
)

(event Custom|Clients_Timer
  ;[0 0.8953 1] Clients Timer
  (CallFunction|RespawnTime)
  (CallFunction|ServerRespawn))

(event Custom|ServerRespawn
  ;[0 0.1291 1] Respawn Pack
)

(event EventBeginPlay
  ;[0.9495 1 0] Beginplay
  (Actor|SetOwner (Game|GetGameMode))
  ;[0 0.1291 1] Respawn Pack
  (if (== (Variables|Default|GetTimer) 0)
    (Variables|Default|SetTimer 10)
    (bind _healthpack (Variables|Default|GetHealthPack)
      (:then
        (Actor|DestroyActor _healthpack))
      (:else
        _))
    (bind _returnvalue (Game|SpawnActorfromClass "/Game/Blueprints/Pick-Ups/BP_HealthPickup.BP_HealthPickup_C" (Transformation|GetActorTransform) "AdjustIfPossibleButAlwaysSpawn" 0 0))
    (Variables|Default|SetHealthPack _returnvalue)))

(fn ConstructionScript)

(fn RespawnTime
  (Math|Integer|DecrementInt (Variables|Default|GetTimer)
    (:%20%20
      (Rendering|Components|TextRender|SetText (Variables|Default|GetTextRender) (Utilities|Text|ToText(Integer) (Variables|Default|GetTimer)))
      (if (== (Variables|Default|GetTimer) 0)
        (return)))))