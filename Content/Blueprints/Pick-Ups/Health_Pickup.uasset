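; Health pickup actor that restores an overlapping, living BP_CharacterMaster to full health.
; Overlap calls SV_RestoreHealth, which sets Health to MaxHealth if below it, triggers the character's update and plays a 2D sound.
; The pickup destroys itself shortly after overlap, even at full health, or expires on a lifespan set at BeginPlay.
; The OnRep_Heal function is empty.
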(event Custom|SV_RestoreHealth
  (params (Object :type Object%20Object%20Reference))
  (bind _as_bp_character_master (Variables|Default|GetAs%20BP%20Character%20Master))
  (bind _as_bp_character_master_2 (Variables|Default|GetAs%20BP%20Character%20Master))
  ;[0 0 0] Heal
  (Utilities|FlowControl|Sequence
    (:then_0
      (if (< (Variables|/Game/TrueFPS/Characters/BP_CharacterMaster.BP_CharacterMaster_C|GetHealth _as_bp_character_master_2) (Variables|/Game/TrueFPS/Characters/BP_CharacterMaster.BP_CharacterMaster_C|GetMaxHealth _as_bp_character_master_2))
        (if (not (Variables|/Game/TrueFPS/Characters/BP_CharacterMaster.BP_CharacterMaster_C|GetDead? (Variables|Default|GetAs%20BP%20Character%20Master)))
          (Variables|/Game/TrueFPS/Characters/BP_CharacterMaster.BP_CharacterMaster_C|SetHealth _as_bp_character_master (Variables|/Game/TrueFPS/Characters/BP_CharacterMaster.BP_CharacterMaster_C|GetMaxHealth _as_bp_character_master))
          (Default|CallUpdate _as_bp_character_master))))
    (:then_1
      (CallFunction|PickupSound))))

(event Custom|PickupSound
  ;[0 0 0] Pickup Sound
  (Audio|PlaySound2D "/Game/TrueFPS/Effects/Sounds/Pickups/SCue_Pickup_Health.SCue_Pickup_Health" 0.5 1.0 0.0 0 0))

(event EventBeginPlay
  ;[0 0 0] Beginplay
  (Variables|Default|GetHealthPack
    (:then
      (Actor|SetLifeSpan 15.0))
    (:else)))

(event Collision|EventActorBeginOverlap
  (params (OtherActor :type Actor%20Object%20Reference))
  ;[0 0 0] Actor Overlap
  (bind _asbp_character_master (Utilities|Casting|CastToBP_CharacterMaster OtherActor))
  (bind _output_get (Variables|Default|SetAs%20BP%20Character%20Master _asbp_character_master))
  (if (not (Variables|/Game/TrueFPS/Characters/BP_CharacterMaster.BP_CharacterMaster_C|GetDead? _output_get))
    (Utilities|FlowControl|Sequence
      (:then_0
        (CallFunction|SVRestoreHealth OtherActor))
      (:then_1
        (Variables|Default|GetHealthPack
          (:then
            (Utilities|FlowControl|Delay 0.3)
            (Actor|DestroyActor))
          (:else))))))

(fn ConstructionScript)

(fn OnRepHeal)