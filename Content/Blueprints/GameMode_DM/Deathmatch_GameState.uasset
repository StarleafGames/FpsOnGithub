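; Deathmatch game state that runs repeating timed rounds, hard-set to 1v1, and tracks Alpha and Bravo team scores.
; On authority, a looping pre-match countdown activates the game and hands off to a match countdown.
; A round restarts when time expires or either score exceeds a threshold that rises each restart, while scores carry over.
; Getters expose active state, remaining time and team scores; game type, player score and team getters are stubs.
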(event Custom|DecrementMatchTimer
  ;[0 0.02733 1] Start Match Timer
  (bind _result (Math|Integer|DecrementInt (Variables|Default|GetMatchTime))
    (:%20%20
      (if (or (<= _result 0) (or (> (Variables|Default|GetTeamAlphaScore) (Variables|Default|GetTeamScoreNeededForReset)) (> (Variables|Default|GetTeamBravoScore) (Variables|Default|GetTeamScoreNeededForReset)))) ; End IF Match Time = 0 \nOR\nTeam Gets A Kill
        (Variables|Default|SetGameIsActive false)
        (Utilities|Time|ClearandInvalidateTimerbyHandle (Variables|Default|GetMatchTimer))
        (switch Utilities|FlowControl|Switch|SwitchonGameType (Variables|Default|GetGameType)
          (:NewEnumerator1
            (CallFunction|RestartRound)))))))

(event Custom|DecrementPreMatchTimer
  ;[0 0.02733 1] Start Pre Match Timer
  (bind _result (Math|Integer|DecrementInt (Variables|Default|GetPreMatchTime))
    (:%20%20
      (if (== _result 0) ; IF prematchtimer = 0
        (Variables|Default|SetGameIsActive true)
        (Utilities|Time|ClearandInvalidateTimerbyHandle (Variables|Default|GetPreMatchTimer)) ; Stop prematch timer
        ;[0 0.02733 1] Match Timer
        (bind _returnvalue (Utilities|Time|SetTimerbyEvent (delegate Custom|DecrementMatchTimer) 1.0 true))
        (Variables|Default|SetMatchTimer _returnvalue)))))

(event Custom|Restart%20Round
  ;[0 0.02733 1] Restart Round
  (Variables|Default|SetPreMatchTime (Variables|DefaultValues|GetDefaultPreMatchTime))
  (Variables|Default|SetMatchTime (Variables|DefaultValues|GetDefaultMatchTime))
  (Math|Integer|IncrementInt (Variables|Default|GetTeamScoreNeededForReset) ; Add 1 Every Reset
    (:%20%20
      ;[0 0.02733 1] Pre Match Timer
      (Networking|SwitchHasAuthority ; To Make Sure Server Has Authority
        (:Authority
          (bind _returnvalue (Utilities|Time|SetTimerbyEvent (delegate Custom|DecrementPreMatchTimer) 1.0 true))
          (Variables|Default|SetPreMatchTimer _returnvalue))))))

(event EventSetGameType
  (params (GameType :type GameType%20Enum :default "NewEnumerator0")))

(event EventIncrementTeamScore
  (params (Team :type TeamNames%20Enum :default "NewEnumerator0"))
  ;[0 0.02733 1] Increment Team Score
  (switch Utilities|FlowControl|Switch|SwitchonTeamNames Team
    (:NewEnumerator0
      (Math|Integer|IncrementInt (Variables|Default|GetTeamAlphaScore)))
    (:NewEnumerator1
      (Math|Integer|IncrementInt (Variables|Default|GetTeamBravoScore)))))

(event EventBeginPlay
  ;[0 0.02733 1] Beginplay
  ;[0 0.02733 1] Set GameType
  (bind _output_get (Variables|Default|SetGameType "NewEnumerator1"))
  (switch Utilities|FlowControl|Switch|SwitchonGameType _output_get
    (:NewEnumerator1
      ;[0 0.02733 1] Set Gameplay Variables
      (bind (_prematchoutput _matchtimeoutput _alphascoreoutput _bravoscoreoutput) (Utilities|SetGameTypeValues 5 60))
      (Utilities|SetDefaultGameTypeValues _prematchoutput _matchtimeoutput _alphascoreoutput _bravoscoreoutput)
      ;[0 0.02733 1] Pre Match Timer
      (Networking|SwitchHasAuthority ; To Make Sure Server Has Authority
        (:Authority
          (bind _returnvalue (Utilities|Time|SetTimerbyEvent (delegate Custom|DecrementPreMatchTimer) 1.0 true))
          (Variables|Default|SetPreMatchTimer _returnvalue))))))

(fn ConstructionScript)

(fn GetGameIsActive
  (return (Variables|Default|GetGameIsActive)))

(fn GetGameTimeRemaining
  (if (Variables|Default|GetGameIsActive)
    (return (Variables|Default|GetMatchTime))
    (else
      (return (Variables|Default|GetPreMatchTime)))))

(fn GetGameType
  (return "NewEnumerator0"))

(fn GetPlayerScore
  (return 0))

(fn GetTeam
  (return "NewEnumerator0" ""))

(fn GetTeamScore
  (return (Variables|Default|GetTeamAlphaScore) (Variables|Default|GetTeamBravoScore)))