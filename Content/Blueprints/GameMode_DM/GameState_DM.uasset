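; Deathmatch GameState that runs timed rounds and tracks Alpha and Bravo team scores.
; An authority-only looping timer counts down pre-match, then activates the game and starts the match countdown.
; When match time expires or either team scores, RestartRound resets times and scores, teleports itself to a random PlayerStart and restarts the pre-match timer.
; Getters expose active state, remaining time and team scores, while player score and team return fixed values.
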(event Custom|DecrementMatchTimer
  ;[0 0 0] Start Match Timer
  (bind _result (Math|Integer|DecrementInt (Variables|Default|GetMatchTime))
    (:%20%20
      (if (or (<= _result 0) (or (> (Variables|Default|GetTeamAlphaScore) 0) (> (Variables|Default|GetTeamBravoScore) 0)))
        (Variables|Default|SetGameIsActive false)
        (Utilities|Time|ClearandInvalidateTimerbyHandle (Variables|Default|GetMatchTimer))
        (CallFunction|RestartRound)))))

(event Custom|DecrementPreMatchTimer
  ;[0 0 0] Start Pre Match Timer
  (bind _result (Math|Integer|DecrementInt (Variables|Default|GetPreMatchTime))
    (:%20%20
      (if (== _result 0) ; IF prematchtimer = 0
        (Variables|Default|SetGameIsActive true)
        (Utilities|Time|ClearandInvalidateTimerbyHandle (Variables|Default|GetPreMatchTimer)) ; Stop prematch timer
        ;[0 0 0] Match Timer
        (bind _returnvalue (Utilities|Time|SetTimerbyEvent (delegate Custom|DecrementMatchTimer) 1.0 true))
        (Variables|Default|SetMatchTimer _returnvalue)))))

(event Custom|Restart%20Round
  (Variables|Default|SetPreMatchTime 5)
  (Variables|Default|SetMatchTime 22)
  (Variables|Default|SetTeamAlphaScore 0)
  (Variables|Default|SetTeamBravoScore 0)
  (bind _outactors (Actor|GetAllActorsOfClass "/Script/Engine.PlayerStart"))
  (Transformation|Teleport (.location (Transformation|GetActorTransform (.OutItem (Utilities|Array|Random _outactors)))) "0, 0, 0")
  ;[0 0 0] Pre Match Timer
  (Networking|SwitchHasAuthority
    (:Authority
      (bind _returnvalue (Utilities|Time|SetTimerbyEvent (delegate Custom|DecrementPreMatchTimer) 1.0 true))
      (Variables|Default|SetPreMatchTimer _returnvalue))))

(event EventIncrementTeamScore
  (params (Team :type TeamNames%20Enum :default "NewEnumerator0"))
  ;[0 0 0] Increment Team Score
  (switch Utilities|FlowControl|Switch|SwitchonTeamNames Team
    (:NewEnumerator0
      (Math|Integer|IncrementInt (Variables|Default|GetTeamAlphaScore)))
    (:NewEnumerator1
      (Math|Integer|IncrementInt (Variables|Default|GetTeamBravoScore)))))

(event EventBeginPlay
  ;[0 0 0] Beginplay
  ;[0 0 0] Pre Match Timer
  (Networking|SwitchHasAuthority
    (:Authority
      (bind _returnvalue (Utilities|Time|SetTimerbyEvent (delegate Custom|DecrementPreMatchTimer) 1.0 true))
      (Variables|Default|SetPreMatchTimer _returnvalue))))

(fn ConstructionScript)

(fn GetGameIsActive
  (return (Variables|Default|GetGameIsActive)))

(fn GetGameTimeRemaining
  (if (Variables|Default|GetGameIsActive)
    (return (Variables|Default|GetMatchTime))
    (else
      (return (Variables|Default|GetPreMatchTime)))))

(fn GetPlayerScore
  (return 0))

(fn GetTeam
  (return "NewEnumerator0" ""))

(fn GetTeamScore
  (return (Variables|Default|GetTeamAlphaScore) (Variables|Default|GetTeamBravoScore)))