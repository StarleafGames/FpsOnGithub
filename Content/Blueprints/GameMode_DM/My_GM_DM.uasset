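; Deathmatch game mode that alternately assigns joining players to two colored teams and spawns their pawns.
; After a short delay, each player possesses a team-colored BP_Smoke spawned at a random PlayerStart, regardless of team.
; RespawnRequested is empty; team-tagged start lookup and a respawn with temporary damage protection are left disabled.
; Game state, score and team getters are stubs returning defaults or nothing.
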(event Custom|RespawnRequested
  (params (Player%20Controller :type Player%20Controller%20Object%20Reference) (Spawn%20Transform :type Transform))
  ;[0 0 0] Respawn Requested
)

(event EventHandleStartingNewPlayer
  (params (NewPlayer :type Player%20Controller%20Object%20Reference))
  ;[1 1 1] Starting New Player
  (Utilities|FlowControl|FlipFlop
    (:A
      (Class|DeathmatchINT|SetTeam(Message) (Variables|/Script/Engine.Controller|GetPlayerState NewPlayer) "NewEnumerator0" "(R=0.000000,G=0.173060,B=1.000000,A=1.000000)"))
    (:B
      (Class|DeathmatchINT|SetTeam(Message) (Variables|/Script/Engine.Controller|GetPlayerState NewPlayer) "NewEnumerator1" "(R=1.000000,G=0.000000,B=0.008450,A=1.000000)")))
  (Utilities|FlowControl|Delay 2.0)
  (CallFunction|SpawnNewPlayerPawn NewPlayer))

(event EventSpawnNewPlayerPawn
  (params (PlayerController :type Controller%20Object%20Reference))
  ;[1 1 1] Spawn New Player Pawn
  (bind (_teamname _teamcolor) (Class|DeathmatchINT|GetTeam(Message) (Variables|/Script/Engine.Controller|GetPlayerState PlayerController)))
  (bind _outactors (Actor|GetAllActorsOfClass "/Script/Engine.PlayerStart"))
  (bind _returnvalue (Game|SpawnActorfromClass "/Game/TrueFPS/Characters/BP_Smoke.BP_Smoke_C" (Transformation|GetActorTransform (.OutItem (Utilities|Array|Random _outactors))) "AdjustIfPossibleButAlwaysSpawn" PlayerController 1e+02 _teamcolor 0))
  (Pawn|Possess PlayerController _returnvalue))

(fn ConstructionScript)

(fn GetGameIsActive
  (return false))

(fn GetGameTimeRemaining
  (return 0))

(fn GetPlayerScore
  (return 0))

(fn GetTeam)

(fn GetTeamScore
  (return 0 0))