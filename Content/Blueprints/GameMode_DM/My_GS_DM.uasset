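; Game state for the DM mode, tracking Alpha and Bravo team scores and the match clock.
; On the authority, BeginPlay starts a one-second looping pre-match countdown, which at zero sets the game active and starts the match countdown.
; When match time runs out, the game goes inactive and the timer is cleared.
; GetTeam only returns a fixed Alpha name and black color.
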(event Custom|DecrementMatchTimer
  ;[0 0 0] Match Timer
  (bind _result (Math|Integer|DecrementInt (Variables|Default|GetMatchTime))
    (:%20%20
      (if (<= _result 0)
        (Variables|Default|SetGameIsActive false)
        (Utilities|Time|ClearandInvalidateTimerbyHandle (Variables|Default|GetMatchTimer))))))

(event Custom|DecrementPreMatchTimer
  ;[0 0 0] Pre Match Timer
  (bind _result (Math|Integer|DecrementInt (Variables|Default|GetPreMatchTime))
    (:%20%20
      (if (== _result 0)
        (Variables|Default|SetGameIsActive true)
        (Utilities|Time|ClearandInvalidateTimerbyHandle (Variables|Default|GetPreMatchTimer))
        ;[0 0 0] Match Timer
        (bind _returnvalue (Utilities|Time|SetTimerbyEvent (delegate Custom|DecrementMatchTimer) 1.0 true))
        (Variables|Default|SetMatchTimer _returnvalue)))))

(event EventIncrementTeamScore
  (params (Team :type TeamNames%20Enum :default "NewEnumerator0"))
  ;[0 0 0] Increment Team Score
  (switch Utilities|FlowControl|Switch|SwitchonTeamNames Team
    (:NewEnumerator0
      (Math|Integer|IncrementInt (Variables|Default|GetTeamAlphaScore)))
    (:NewEnumerator1
      (Math|Integer|IncrementInt (Variables|Default|GetTeamBravoScore)))))

(event EventBeginPlay
  ;[0 0 0] Beginplay
  (Networking|SwitchHasAuthority
    (:Authority
      (bind _returnvalue (Utilities|Time|SetTimerbyEvent (delegate Custom|DecrementPreMatchTimer) 1.0 true))
      (Variables|Default|SetPreMatchTimer _returnvalue))))

(fn ConstructionScript)

(fn GetTeam
  (return "NewEnumerator0" ""))