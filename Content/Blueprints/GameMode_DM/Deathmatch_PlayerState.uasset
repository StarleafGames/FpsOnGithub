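; Deathmatch player state that tracks one player's personal score along with a team name and color.
; Events increment the score and set the team, getters return both, and BeginPlay caches the pawn as a BP_CharacterMaster.
; The match-level getters for active state, time remaining, game type and team scores are stubs returning fixed default values.
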(event EventSetTeam
  (params (TeamName :type TeamNames%20Enum :default "NewEnumerator0") (TeamColor :type Linear%20Color%20Structure))
  ;[0 0 0] Set Team Name And Color
  (Variables|Default|SetTeam%20Name TeamName)
  (Variables|Default|SetTeam%20Color TeamColor))

(event EventIncrementPlayerScore
  ;[0 0 0] Increment Player Personal Score
  (Math|Integer|IncrementInt (Variables|Default|GetPersonalScore)))

(event EventBeginPlay
  ;[0 0 0] Beginplay
  ;[0 0 0] Cast to CharacterMaster
  (bind _asbp_character_master (Utilities|Casting|CastToBP_CharacterMaster (PlayerState|GetPawn)))
  (Variables|Default|SetAs%20BP%20Character%20Master _asbp_character_master))

(fn ConstructionScript)

(fn GetGameIsActive
  (return false))

(fn GetGameTimeRemaining
  (return 0))

(fn GetGameType
  (return "NewEnumerator0"))

(fn GetPlayerScore
  (return (Variables|Default|GetPersonalScore)))

(fn GetTeam
  (return (Variables|Default|GetTeam%20Name) (Variables|Default|GetTeam%20Color)))

(fn GetTeamScore
  (return 0 0))