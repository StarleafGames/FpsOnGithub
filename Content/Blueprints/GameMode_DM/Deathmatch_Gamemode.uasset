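; Deathmatch game mode that spawns a BP_Smoke pawn at a random PlayerStart and possesses it for each joining player.
; PostLogin tracks controllers, though its spawn sits inside the loop over all of them; SpawnNewPlayerPawn repeats the spawn for a given controller.
; HandleStartingNewPlayer alternates two colored teams via FlipFlop, messaging the PlayerState.
; Game-state and score getters are stubs; BP_PlayerSpawn validity-check spawning is unwired.
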(event EventPostLogin
  (params (NewPlayer :type Player%20Controller%20Object%20Reference))
  (bind _playerscontrollersarray (Variables|Default|GetPlayersControllersArray))
  ;[0 0.02733 1] On Post Login
  (Utilities|Array|AddUnique _playerscontrollersarray NewPlayer)
  (for _array_element _playerscontrollersarray
    (Variables|Default|SetPlayerCountNumber (Utilities|Array|Length _playerscontrollersarray))
    (Utilities|FlowControl|Delay 1.0)
    ;[0 0.02733 1] Spawn New Player Pawn
    (bind _outactors (Actor|GetAllActorsOfClass "/Script/Engine.PlayerStart"))
    (bind _returnvalue (Game|SpawnActorfromClass "/Game/TrueFPS/Characters/BP_Smoke.BP_Smoke_C" (Transformation|GetActorTransform (.OutItem (Utilities|Array|Random _outactors))) "AdjustIfPossibleButAlwaysSpawn" NewPlayer 1e+02 "(R=0.000000,G=0.000000,B=0.000000,A=0.000000)" 0))
    (Pawn|Possess NewPlayer _returnvalue)
    (Utilities|FlowControl|Delay 0.3)))

(event EventHandleStartingNewPlayer
  (params (NewPlayer :type Player%20Controller%20Object%20Reference))
  ;[0 0.02733 1] Starting New Player
  (Utilities|FlowControl|Delay 0.2)
  (Development|PrintString "New Player Starting" false)
  (Utilities|FlowControl|FlipFlop
    (:A
      (Class|DeathmatchINT|SetTeam(Message) (Variables|/Script/Engine.Controller|GetPlayerState NewPlayer) "NewEnumerator0" "(R=0.000000,G=0.173060,B=1.000000,A=1.000000)"))
    (:B
      (Class|DeathmatchINT|SetTeam(Message) (Variables|/Script/Engine.Controller|GetPlayerState NewPlayer) "NewEnumerator1" "(R=1.000000,G=0.000000,B=0.008450,A=1.000000)")))
  (Utilities|FlowControl|Delay 2.0))

(event EventSpawnNewPlayerPawn
  (params (PlayerController :type Controller%20Object%20Reference))
  ;[0 0.02733 1] Spawn New Player Pawn
  (Class|DeathmatchINT|GetTeam(Message) (Variables|/Script/Engine.Controller|GetPlayerState PlayerController))
  (bind _outactors (Actor|GetAllActorsOfClass "/Script/Engine.PlayerStart"))
  (bind _returnvalue (Game|SpawnActorfromClass "/Game/TrueFPS/Characters/BP_Smoke.BP_Smoke_C" (Transformation|GetActorTransform (.OutItem (Utilities|Array|Random _outactors))) "AdjustIfPossibleButAlwaysSpawn" PlayerController 1e+02 "(R=0.000000,G=0.000000,B=0.000000,A=0.000000)" 0))
  (Pawn|Possess PlayerController _returnvalue))

(fn ConstructionScript)

(fn GameIsInactive
  (return false))

(fn GetGameIsActive
  (return false))

(fn GetGameTimeRemaining
  (return 0))

(fn GetGameType
  (return "NewEnumerator0"))

(fn GetPlayerScore
  (return 0))

(fn GetTeam)

(fn GetTeamScore
  (return 0 0))