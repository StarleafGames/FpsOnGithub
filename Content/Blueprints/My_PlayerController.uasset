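; Player controller that handles the pause-style menu, death and respawn flow, sniper overlay and pawn input toggling.
; P flip-flops the escape menu along with cursor and input mode; sniper overlay creation and input toggles run only on the local controller.
; Death waits, unpossesses, requests a respawn through Main_GM, then refreshes the HUD.
; HUD setup, death screen and sniper overlay removal are disabled; score and post-login events are empty.
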(event Custom|ClientPostLogin)

(event Custom|CE_DeathHud
  ;[0 0 0] Death HUD
  (Utilities|FlowControl|Delay 3.0)
  (Pawn|UnPossess)
  (Utilities|FlowControl|Delay 1.0)
  (CallFunction|RespawnPawn)
  (CallFunction|CERefreshHUD))

(event Custom|Net_Scores
  ;[0 0 0] Score Count
)

(event Custom|SniperHud
  (if (Pawn|IsLocalController)
    (bind _returnvalue (UserInterface|CreateWidget "/Game/TrueFPS/UI/Other/SniperUI/Sniper_UI.Sniper_UI_C" self))
    (bind _output_get (Variables|Default|SetSniperUI _returnvalue))
    (UserInterface|Viewport|AddtoViewport _output_get 0)))

(event Custom|RemoveSniperHUD
  (if (Pawn|IsLocalController)
    (Widget|RemovefromParent (Variables|Default|GetSniperUI))))

(event Custom|CE_RefreshHUD
  ;[0 0 0] Refresh HUD
  (Default|CallRespawned))

(event Custom|RespawnPawn
  (params (Spawn%20Transform :type Transform))
  ;[0 0 0] Respawn Pawn
  (bind _asmain_gm (Utilities|Casting|CastToMain_GM (Game|GetGameMode)))
  (Default|RespawnRequested _asmain_gm self Spawn%20Transform))

(event Custom|InputOn
  (if (Pawn|IsLocalController)
    (Input|EnableInput (Pawn|GetControlledPawn) self)))

(event Custom|InputOff
  (if (Pawn|IsLocalController)
    (Input|DisableInput (Pawn|GetControlledPawn) self)))

(event Input|KeyboardEvents|P
  (params (Key :type Key%20Structure :default "None"))
  ;[0 0 0] Esc Menu [P]
  (:Pressed
    (Utilities|FlowControl|FlipFlop
      (:A
        (bind _returnvalue (UserInterface|CreateWidget "/Game/TrueFPS/UI/Other/EscMenu_UI1.EscMenu_UI1_C" self))
        (bind _output_get (Variables|Default|SetEscmenu2 _returnvalue))
        (UserInterface|Viewport|AddtoViewport _output_get 0)
        (Variables|Default|SetbShowMouseCursor true)
        (Input|SetInputModeGameandUI self _returnvalue "DoNotLock" true))
      (:B
        (Variables|Default|SetbShowMouseCursor false)
        (Input|SetInputModeGameOnly self)
        (Widget|RemovefromParent (Variables|Default|GetEscmenu2))))))

(fn ConstructionScript)

(fn SetupIngameUI)