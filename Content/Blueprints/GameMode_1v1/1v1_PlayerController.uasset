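; Player controller for the 1v1 game mode, managing local UI: the match widget, sniper scope overlay and a developer overlay.
; BeginPlay adds the 1v1 widget and sets game-only input, while key 7 toggles the dev overlay.
; Sniper events add the scope widget and hide the controlled character's mesh from its owner with hidden shadow casting, or make it visible again.
; CE_RefreshHUD calls CallRespawned; the older player HUD creation is disabled.
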(event Custom|SniperHud
  ;[0 0 0] SniperHUD
  (if (Pawn|IsLocalController)
    (bind _returnvalue (UserInterface|CreateWidget "/Game/TrueFPS/UI/Other/SniperUI/Sniper_UI.Sniper_UI_C" self))
    (bind _output_get (Variables|Default|SetSniperUI _returnvalue))
    (UserInterface|Viewport|AddtoViewport _output_get 0)
    (bind _asbp_character_master (Utilities|Casting|CastToBP_CharacterMaster (Pawn|GetControlledPawn)))
    (bind _mesh (Variables|/Script/Engine.Character|GetMesh _asbp_character_master)
      (:then
        (Class|PrimitiveComponent|SetOwnerNoSee _mesh true)
        (Class|PrimitiveComponent|SetCastHiddenShadow _mesh true))
      (:else))))

(event Custom|CE_RefreshHUD
  ;[0 0 0] Refresh HUD
  (Default|CallRespawned))

(event Custom|ShowSniper
  ;[0 0 0] Show Sniper
  (if (Pawn|IsLocalController)
    (bind _asbp_character_master (Utilities|Casting|CastToBP_CharacterMaster (Pawn|GetControlledPawn)))
    (Variables|Default|SetAs%20BP%20Character%20Master _asbp_character_master)
    (Class|PrimitiveComponent|SetOwnerNoSee (Variables|/Script/Engine.Character|GetMesh _asbp_character_master) false)))

(event EventBeginPlay
  ;[0 0 0] Beginplay
  ;[1 1 1] DM UI
  (if (Pawn|IsLocalPlayerController)
    (bind _returnvalue (UserInterface|CreateWidget "/Game/TrueFPS/UI/1v1/1v1_WBP.1v1_WBP_C"))
    (UserInterface|Viewport|AddtoViewport _returnvalue 0)
    (Input|SetInputModeGameOnly self)))

(event Input|KeyboardEvents|7
  (params (Key :type Key%20Structure :default "None"))
  ;[0 0 0] Dev Overlay
  (:Pressed
    (Utilities|FlowControl|FlipFlop
      (:A
        (if (Pawn|IsLocalPlayerController)
          (bind _returnvalue (UserInterface|CreateWidget "/Game/TrueFPS/UI/Other/WBP_DevOverlay.WBP_DevOverlay_C" self))
          (bind _output_get (Variables|Default|SetDevUI _returnvalue))
          (UserInterface|Viewport|AddtoViewport _output_get 0)))
      (:B
        (Widget|RemovefromParent (Variables|Default|GetDevUI))
        (Input|SetInputModeGameOnly self)
        (if (Variables|Default|GetbShowMouseCursor)
          (Variables|Default|SetbShowMouseCursor false))))))

(fn ConstructionScript)