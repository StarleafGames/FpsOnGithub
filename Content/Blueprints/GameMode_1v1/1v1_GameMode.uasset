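; Game mode for 1v1 matches that assigns joining players to one of two colored teams and spawns their BP_Smoke pawns.
; PostLogin and HandleStartingNewPlayer each alternate teams via their own FlipFlop, set PlayerState through an interface message, then spawn after a delay.
; Spawning picks a random PlayerStart and possesses a team-colored pawn; team-tagged start lookup is disabled.
; Game state, score, time and team getters return placeholder values.
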(event EventHandleStartingNewPlayer
  (params (NewPlayer :type Player%20Controller%20Object%20Reference))
  ;[0 0.02733 1] Starting New Player
  (Utilities|FlowControl|FlipFlop
    (:A
      (Class|1v1INT|SetTeam1v1(Message) (Variables|/Script/Engine.Controller|GetPlayerState NewPlayer) "NewEnumerator0" "(R=0.000000,G=0.216702,B=1.000000,A=1.000000)"))
    (:B
      (Class|1v1INT|SetTeam1v1(Message) (Variables|/Script/Engine.Controller|GetPlayerState NewPlayer) "NewEnumerator1" "(R=1.000000,G=0.000000,B=0.047313,A=1.000000)")))
  (Utilities|FlowControl|Delay 2.0)
  (CallFunction|SpawnNewPlayerPawn1v1 NewPlayer))

(event EventPostLogin
  (params (NewPlayer :type Player%20Controller%20Object%20Reference))
  (bind _playerscontrollersarray (Variables|Default|GetPlayersControllersArray))
  ;[0 0.02733 1] On Post Login
  (Utilities|Array|AddUnique _playerscontrollersarray NewPlayer)
  (bind _output_get (Variables|Default|SetPlayerCountNumber (Utilities|Array|Length _playerscontrollersarray)))
  (Variables|Default|SetPlayerCountArray (Utilities|Array|MakeArray _output_get))
  ;[0 0.02733 1] Starting New Player
  (Utilities|FlowControl|FlipFlop
    (:A
      (Class|1v1INT|SetTeam1v1(Message) (Variables|/Script/Engine.Controller|GetPlayerState NewPlayer) "NewEnumerator0" "(R=0.000000,G=0.216702,B=1.000000,A=1.000000)"))
    (:B
      (Class|1v1INT|SetTeam1v1(Message) (Variables|/Script/Engine.Controller|GetPlayerState NewPlayer) "NewEnumerator1" "(R=1.000000,G=0.000000,B=0.047313,A=1.000000)")))
  (Utilities|FlowControl|Delay 2.0)
  (CallFunction|SpawnNewPlayerPawn1v1 NewPlayer))

(event EventSpawnNewPlayerPawn1v1
  (params (PlayerController :type Controller%20Object%20Reference))
  ;[0 0.02733 1] Spawn New Player Pawn
  (bind (_teamname _teamcolor) (Class|1v1INT|GetTeam1v1(Message) (Variables|/Script/Engine.Controller|GetPlayerState PlayerController)))
  (bind _outactors (Actor|GetAllActorsOfClass "/Script/Engine.PlayerStart"))
  (bind _returnvalue (Game|SpawnActorfromClass "/Game/TrueFPS/Characters/BP_Smoke.BP_Smoke_C" (Transformation|GetActorTransform (.OutItem (Utilities|Array|Random _outactors))) "AdjustIfPossibleButAlwaysSpawn" PlayerController 1e+02 _teamcolor 0))
  (Pawn|Possess PlayerController _returnvalue))

(fn ConstructionScript)

(fn GetGameIsActive1v1
  (return false))

(fn GetGameTimeRemaining1v1
  (return 0))

(fn GetPlayerScore1v1
  (return 0))

(fn GetTeam1v1
  (return "NewEnumerator0" ""))

(fn GetTeamScore1v1
  (return 0 0))