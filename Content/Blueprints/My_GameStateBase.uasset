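; My_GameStateBase is a game state Blueprint that triggers an on-screen countdown.
; On BeginPlay it caches the first player controller as My_PlayerController and its controlled pawn as BP_CharacterMaster.
; Server_StartCountdown hands off to a client countdown event, with names suggesting a server-to-client RPC pattern.
; Client_Countdown creates a Countdown_WBP widget and adds it to the viewport.
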(event Custom|Client_Countdown
  (bind _returnvalue (UserInterface|CreateWidget "/Game/TrueFPS/UI/Game/Countdown_WBP.Countdown_WBP_C"))
  (UserInterface|Viewport|AddtoViewport _returnvalue 0))

(event Custom|Server_StartCountdown
  (CallFunction|ClientCountdown))

(event EventBeginPlay
  (bind _asmy_player_controller (Utilities|Casting|CastToMy_PlayerController (Game|GetPlayerController 0)))
  (bind _output_get (Variables|Default|SetAs%20My%20Player%20Controller _asmy_player_controller))
  (bind _asbp_character_master (Utilities|Casting|CastToBP_CharacterMaster (Pawn|GetControlledPawn _output_get)))
  (Variables|Default|SetAs%20BP%20Character%20Master _asbp_character_master))

(fn ConstructionScript)