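; Game instance for a Deathmatch game that hosts multiplayer sessions and shows a loading screen.
; HOSTSESSION creates a session with configurable connections and LAN use, then on success shows the loading screen, waits briefly and opens the chosen level as a listen server.
; The loading screen widget is created once, cached and given UI-only input.
; Game-state, score, team and timer getters are stubs returning defaults.
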(event Custom|HOST%20SESSION
  (params (PublicConnections :type Integer) (bUseLAN :type Boolean) (LevelName :type Name))
  ;[0 0 0] Host Session def
  (|Session (Game|GetPlayerController 0) PublicConnections bUseLAN
    (:OnSuccess
      (CallFunction|CEShowLoadingScreen)
      (Utilities|FlowControl|Delay 4.0)
      (Game|OpenLevel(byName) LevelName true "listen"))
    (:OnFailure
      (Development|PrintString "Failed to created a session"))))

(event Custom|CE_ShowLoadingScreen
  (bind _returnvalue (Game|GetPlayerController 0))
  ;[0 0 0] Show Loading Screen
  (Utilities|IsValid (Variables|Default|GetLoadingScreenUI)
    (:Is%20Valid
      _)
    (:Is%20Not%20Valid
      (bind _returnvalue_2 (UserInterface|CreateWidget "/Game/TrueFPS/UI/MainMenu/WBP_LoadingScreen.WBP_LoadingScreen_C" _returnvalue))
      (Variables|Default|SetLoadingScreenUI _returnvalue_2)))
  (UserInterface|Viewport|AddtoViewport (Variables|Default|GetLoadingScreenUI) 0)
  (Input|SetInputModeUIOnly _returnvalue (Variables|Default|GetLoadingScreenUI) "DoNotLock"))

(fn GameIsInactive
  (return false))

(fn GetGameIsActive
  (return false))

(fn GetGameTimeRemaining
  (return 0))

(fn GetGameType
  (return "NewEnumerator0"))

(fn GetPlayerScore
  (return 0))

(fn GetTeam
  (return "NewEnumerator0" ""))

(fn GetTeamScore
  (return 0 0))