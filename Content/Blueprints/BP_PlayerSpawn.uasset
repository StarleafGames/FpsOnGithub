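; BP_PlayerSpawn is a player spawn point actor that tracks whether its location is currently free.
; A ValidSpawn flag starts true, goes false when something overlaps the actor or its BoxCollision, and returns true when an overlap ends.
; It keeps no overlap count, so any single exit marks it valid; actor overlaps also print debug messages.
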(event OnComponentBeginOverlap(BoxCollision)
  (params (OverlappedComponent :type Primitive%20Component%20Object%20Reference) (OtherActor :type Actor%20Object%20Reference) (OtherComp :type Primitive%20Component%20Object%20Reference) (OtherBodyIndex :type Integer) (bFromSweep :type Boolean) (SweepResult :type Hit%20Result%20Structure%20%28by%20ref%29))
  (Variables|Default|SetValidSpawn false))

(event OnComponentEndOverlap(BoxCollision)
  (params (OverlappedComponent :type Primitive%20Component%20Object%20Reference) (OtherActor :type Actor%20Object%20Reference) (OtherComp :type Primitive%20Component%20Object%20Reference) (OtherBodyIndex :type Integer))
  (Variables|Default|SetValidSpawn true))

(event EventBeginPlay
  (Variables|Default|SetValidSpawn true))

(event Collision|EventActorBeginOverlap
  (params (OtherActor :type Actor%20Object%20Reference))
  (Variables|Default|SetValidSpawn false)
  (Development|PrintString "Not Valid Spawn"))

(event EventTick
  (params (DeltaSeconds :type Float%20%28single-precision%29)))

(event Collision|EventActorEndOverlap
  (params (OtherActor :type Actor%20Object%20Reference))
  (Variables|Default|SetValidSpawn true)
  (Development|PrintString "Valid Spawn"))

(fn ConstructionScript)