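; Game mode that starts a multiplayer match and handles player respawns.
; PostLogin records controllers and runs a looping timer that, once more than one player connects, readies each with a BP_Smoke pawn, HUD and match timer.
; Respawn requests pass a DoOnce gate, expire the old pawn, possess a new one and make it temporarily invulnerable.
; Spawn points are randomly picked named PlayerStarts.
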(event Custom|CE_WaitForPlayers
  ;[0 0 0] Wait For Players
  (if (Variables|Default|GetDebug)
    (Development|PrintString (Utilities|String|Append "Player's Connected: " (Utilities|String|ToString(Integer) (Class|GameplayStatics|GetNumPlayerControllers))) true true "(R=0.000000,G=0.660000,B=1.000000,A=1.000000)" 1.0))
  (if (> (Class|GameplayStatics|GetNumPlayerControllers) 1)
    (if (Variables|Default|GetDebug)
      (Development|PrintString "WaitingToStart" true true "(R=0.000000,G=0.660000,B=1.000000,A=1.000000)" 3.0))
    (for (_ _array_index) (Variables|Default|GetPlayerControllerList)
      (bind _asmy_player_controller (Utilities|Casting|CastToMy_PlayerController (Game|GetPlayerController _array_index)))
      (bind _output_get (Variables|Default|SetAs%20My%20Player%20Controller _asmy_player_controller))
      (CallFunction|PlayersReady)
      (Default|OCPlayerHUD _output_get)
      (Utilities|Time|ClearandInvalidateTimerbyHandle (Variables|Default|GetWaitingForPlayersTimer))
      (Development|PrintString "Start!")
      (Default|MatchTimer (Variables|Default|GetAs%20My%20Player%20Controller)))
    (elif (Variables|Default|GetDebug)
      (Development|PrintString "WaitingForPlayers" true true "(R=0.000000,G=0.660000,B=1.000000,A=1.000000)" 1.0))))

(event Custom|Players_Ready
  (bind _as_my_player_controller (Variables|Default|GetAs%20My%20Player%20Controller))
  ;[0 0 0] Players Ready
  (Variables|Default|SetReadyToStartMatch true)
  (bind _returnvalue (Game|SpawnActorfromClass "/Game/TrueFPS/Characters/BP_Smoke.BP_Smoke_C" (CallFunction|PlayerStartRespawns _as_my_player_controller) "AlwaysSpawn" 0 1e+02 0))
  (Pawn|Possess _as_my_player_controller _returnvalue))

(event Custom|RespawnRequested
  (params (Player%20Controller :type Player%20Controller%20Object%20Reference) (Spawn%20Transform :type Transform))
  (bind _returnvalue (Pawn|GetControlledPawn Player%20Controller))
  ;[0 0 0] Respawn Requested
  (Utilities|IsValid Player%20Controller
    (:Is%20Valid
      (Utilities|FlowControl|DoOnce false :!label _label
        (:Completed
          (Utilities|IsValid _returnvalue
            (:Is%20Valid
              (Actor|SetLifeSpan _returnvalue 5.0))
            (:Is%20Not%20Valid
              _))
          (bind _returnvalue_2 (Game|SpawnActorfromClass "/Game/TrueFPS/Characters/BP_Smoke.BP_Smoke_C" (CallFunction|PlayerStartRespawns Player%20Controller) "AlwaysSpawn" Player%20Controller 1e+02 0))
          (Utilities|FlowControl|Sequence
            (:then_0
              (Utilities|FlowControl|Delay 0.2)
              (Pawn|Possess Player%20Controller _returnvalue_2)
              (bind _asmy_player_controller (Utilities|Casting|CastToMy_PlayerController Player%20Controller))
              (Default|CERefreshHUD _asmy_player_controller)
              (goto _label Reset))
            (:then_1
              (Variables|/Script/Engine.Actor|SetbCanBeDamaged _returnvalue_2 false)
              (Development|PrintString "Protected")
              (Utilities|FlowControl|Delay 1e+01)
              (Variables|/Script/Engine.Actor|SetbCanBeDamaged _returnvalue_2 true)
              (Development|PrintString "Not Protected"))))))))

(event EventPostLogin
  (params (NewPlayer :type Player%20Controller%20Object%20Reference))
  ;[0 0 0] On Post Login
  (Variables|Default|SetNew%20Player NewPlayer)
  (Utilities|Array|AddUnique (Variables|Default|GetPlayerControllerList) NewPlayer)
  (Variables|Default|SetNumberOfPlayersConnected (+ (Variables|Default|GetNumberOfPlayersConnected) 1))
  (Variables|/Script/Engine.PlayerController|SetbShowMouseCursor NewPlayer false)
  (Input|SetInputModeGameOnly NewPlayer)
  (bind _returnvalue (Utilities|Time|SetTimerbyEvent (delegate Custom|CE_WaitForPlayers) 1.0 true))
  (Variables|Default|SetWaitingForPlayersTimer _returnvalue))

(event EventTick
  (params (DeltaSeconds :type Float%20%28single-precision%29))
  ;[0 0 0] Wait For Players
)

(fn ConstructionScript)

(fn PlayerStartRespawns
  (params (Player :type Controller%20Object%20Reference))
  (return (Transformation|GetActorTransform (Class|GameModeBase|FindPlayerStart (Game|GetGameMode) Player (Utilities|Select :Index (Math|Random|RandomIntegerinRange 0 8) :Option%200 "Respawn" :Option%201 "Respawn1" :Option%202 "Respawn2" :Option%203 "Respawn3" :Option%204 "Respawn4" :Option%205 "Respawn5" :Option%206 "Respawn6" :Option%207 "Respawn7" :Option%208 "Respawn8")))))