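; My_GameInstance is a game instance Blueprint sketching a UI state machine for startup and the main menu, with all of its logic currently disabled.
; Its event and functions are empty or unwired stubs.
; The disabled nodes show TransitionToState guarding against same-state changes and hiding the outgoing menu, while ShowMainMenu lazily creates WBP_MainMenu with UI-only input and a visible cursor.
; A separate disabled node opens the MainMenu level by name.
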(event Custom|ShowMainMenu)

(fn BeginPlayShowMainMenu)

(fn HideUI
  (params (Target :type Widget%20Object%20Reference)))