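; BP_OpticsMaster is an optic attachment Blueprint, apparently the base for sights, that registers itself in its weapon's Optics array.
; On initialization, an optic in the weapon's Other slot switches to its canted distance and is appended, while any other optic overwrites the array's first entry.
; On removal, the canted optic is taken out of the array, while a main optic is replaced by the weapon's FreeSights child actor as fallback.
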(event EventBeginPlay
  (|CallParentFunction) ; This node is disabled and will not be called.\nDrag off pins to build functionality.
)

(event Collision|EventActorBeginOverlap
  (params (OtherActor :type Actor%20Object%20Reference))
  (|CallParentFunction OtherActor) ; This node is disabled and will not be called.\nDrag off pins to build functionality.
)

(event EventTick
  (params (DeltaSeconds :type Float%20%28single-precision%29))
  (|CallParentFunction DeltaSeconds) ; This node is disabled and will not be called.\nDrag off pins to build functionality.
)

(event EventInitializeAttachment
  (params (Weapon :type BP%20Weapon%20Master%20Object%20Reference))
  (bind _optics (Variables|/Game/TrueFPS/Items/Weapons/BP_WeaponMaster.BP_WeaponMaster_C|GetOptics Weapon))
  ;[0 0 0] Set scopes
  (|CallParentFunction Weapon)
  (if (== (Variables|/Game/TrueFPS/Items/Weapons/BP_WeaponMaster.BP_WeaponMaster_C|GetOther Weapon) self)
    (Variables|Default|SetDistance (Variables|Default|GetDistanceCanted))
    (Utilities|Array|Add _optics self)
    (else
      (Utilities|Array|SetArrayElem _optics 0 self true))))

(event EventRemoveAttachment
  (params (Weapon :type BP%20Weapon%20Master%20Object%20Reference))
  (bind _optics (Variables|/Game/TrueFPS/Items/Weapons/BP_WeaponMaster.BP_WeaponMaster_C|GetOptics Weapon))
  ;[0 0 0] Set scopes
  (|CallParentFunction Weapon)
  (Utilities|IsValid Weapon
    (:Is%20Valid
      (if (== (Variables|/Game/TrueFPS/Items/Weapons/BP_WeaponMaster.BP_WeaponMaster_C|GetOther Weapon) self)
        (Utilities|Array|RemoveItem _optics self)
        (else
          (bind _asbp_optics_master (Utilities|Casting|CastToBP_OpticsMaster (Variables|/Script/Engine.ChildActorComponent|GetChildActor (Variables|/Game/TrueFPS/Items/Weapons/BP_WeaponMaster.BP_WeaponMaster_C|GetFreeSights Weapon))))
          (Utilities|Array|SetArrayElem _optics 0 _asbp_optics_master true))))))

(fn ConstructionScript
  (|CallParentFunction))