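; ACOG scope weapon attachment that carries a second optic as a child actor.
; On BeginPlay it disables collision on the child actor.
; After parent initialization, it casts the child to BP_OpticsMaster and inserts it at index 1 of the weapon's Optics array, adding another scope.
; Removing the attachment takes that child optic back out of the array.
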(event EventBeginPlay
  (|CallParentFunction)
  (Collision|SetActorEnableCollision (Variables|/Script/Engine.ChildActorComponent|GetChildActor (Variables|Default|GetChildActor)) false))

(event Collision|EventActorBeginOverlap
  (params (OtherActor :type Actor%20Object%20Reference))
  (|CallParentFunction OtherActor) ; This node is disabled and will not be called.\nDrag off pins to build functionality.
)

(event EventTick
  (params (DeltaSeconds :type Float%20%28single-precision%29))
  (|CallParentFunction DeltaSeconds) ; This node is disabled and will not be called.\nDrag off pins to build functionality.
)

(event EventRemoveAttachment
  (params (Weapon :type BP%20Weapon%20Master%20Object%20Reference))
  ;[1 1 1] Add another scope
  (|CallParentFunction Weapon)
  (bind _asbp_optics_master (Utilities|Casting|CastToBP_OpticsMaster (Variables|/Script/Engine.ChildActorComponent|GetChildActor (Variables|Default|GetChildActor))))
  (Utilities|Array|RemoveItem (Variables|/Game/TrueFPS/Items/Weapons/BP_WeaponMaster.BP_WeaponMaster_C|GetOptics Weapon) _asbp_optics_master))

(event EventInitializeAttachment
  (params (Weapon :type BP%20Weapon%20Master%20Object%20Reference))
  ;[1 1 1] Add another scope
  (|CallParentFunction Weapon)
  (bind _asbp_optics_master (Utilities|Casting|CastToBP_OpticsMaster (Variables|/Script/Engine.ChildActorComponent|GetChildActor (Variables|Default|GetChildActor))))
  (Utilities|Array|Insert (Variables|/Game/TrueFPS/Items/Weapons/BP_WeaponMaster.BP_WeaponMaster_C|GetOptics Weapon) _asbp_optics_master 1))

(fn ConstructionScript
  (|CallParentFunction))