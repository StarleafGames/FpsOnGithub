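; Vertical grip underbarrel weapon attachment that steadies the weapon by reducing camera shake and vertical recoil.
; On attach, it calls the parent, then teleports the weapon's left-hand component to the grip's Scene transform.
; On the authority only, it scales camera shake, pitch recoil and random pitch max by a fixed factor.
; Removal restores the stored relative hand transform and divides those stats by the same factor to undo the change.
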(event EventInitializeAttachment
  (params (Weapon :type BP%20Weapon%20Master%20Object%20Reference))
  (|CallParentFunction Weapon)
  (Transformation|SetWorldTransform (Variables|/Game/TrueFPS/Items/Weapons/BP_WeaponMaster.BP_WeaponMaster_C|GetLeftHand Weapon) (Transformation|GetWorldTransform (Variables|Default|GetScene)) false true)
  (Networking|SwitchHasAuthority
    (:Authority
      (Variables|/Game/TrueFPS/Items/Weapons/BP_WeaponMaster.BP_WeaponMaster_C|SetCameraShakeIntensity Weapon (* (Variables|/Game/TrueFPS/Items/Weapons/BP_WeaponMaster.BP_WeaponMaster_C|GetCameraShakeIntensity Weapon) 0.6))
      (Variables|/Game/TrueFPS/Items/Weapons/BP_WeaponMaster.BP_WeaponMaster_C|SetPitch%20Recoil%20Intensity Weapon (* (Variables|/Game/TrueFPS/Items/Weapons/BP_WeaponMaster.BP_WeaponMaster_C|GetPitch%20Recoil%20Intensity Weapon) 0.6))
      (Variables|/Game/TrueFPS/Items/Weapons/BP_WeaponMaster.BP_WeaponMaster_C|SetRandom%20Pitch%20Max Weapon (* (Variables|/Game/TrueFPS/Items/Weapons/BP_WeaponMaster.BP_WeaponMaster_C|GetRandom%20Pitch%20Max Weapon) 0.6)))))

(event EventRemoveAttachment
  (params (Weapon :type BP%20Weapon%20Master%20Object%20Reference))
  (|CallParentFunction Weapon)
  (Transformation|SetRelativeTransform (Variables|/Game/TrueFPS/Items/Weapons/BP_WeaponMaster.BP_WeaponMaster_C|GetLeftHand Weapon) (Variables|/Game/TrueFPS/Items/Weapons/BP_WeaponMaster.BP_WeaponMaster_C|GetLeftHandRelative Weapon) false true)
  (Networking|SwitchHasAuthority
    (:Authority
      (Variables|/Game/TrueFPS/Items/Weapons/BP_WeaponMaster.BP_WeaponMaster_C|SetCameraShakeIntensity Weapon (/ (Variables|/Game/TrueFPS/Items/Weapons/BP_WeaponMaster.BP_WeaponMaster_C|GetCameraShakeIntensity Weapon) 0.6))
      (Variables|/Game/TrueFPS/Items/Weapons/BP_WeaponMaster.BP_WeaponMaster_C|SetPitch%20Recoil%20Intensity Weapon (/ (Variables|/Game/TrueFPS/Items/Weapons/BP_WeaponMaster.BP_WeaponMaster_C|GetPitch%20Recoil%20Intensity Weapon) 0.6))
      (Variables|/Game/TrueFPS/Items/Weapons/BP_WeaponMaster.BP_WeaponMaster_C|SetRandom%20Pitch%20Max Weapon (/ (Variables|/Game/TrueFPS/Items/Weapons/BP_WeaponMaster.BP_WeaponMaster_C|GetRandom%20Pitch%20Max Weapon) 0.6)))))

(fn ConstructionScript
  (|CallParentFunction))