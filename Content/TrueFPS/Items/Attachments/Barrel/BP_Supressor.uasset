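; Suppressor barrel attachment that quiets a weapon at the cost of performance.
; On initialize, the server swaps the weapon's shot sound and scales down its muzzle velocity, damage and hearing range by fixed multipliers.
; On removal, the server divides those multipliers back out and restores the shot sound from the weapon's class defaults.
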(event EventInitializeAttachment
  (params (Weapon :type BP%20Weapon%20Master%20Object%20Reference))
  (|CallParentFunction Weapon)
  (Networking|SwitchHasAuthority
    (:Authority
      (Variables|/Game/TrueFPS/Items/Weapons/BP_WeaponMaster.BP_WeaponMaster_C|SetShotAudio Weapon "/Game/TrueFPS/Sounds/Sounds/Weapons/Default/SCue_Rifle_Cue1.SCue_Rifle_Cue1")
      (Variables|/Game/TrueFPS/Items/Weapons/BP_WeaponMaster.BP_WeaponMaster_C|SetMuzzleVelocity Weapon (* (Variables|/Game/TrueFPS/Items/Weapons/BP_WeaponMaster.BP_WeaponMaster_C|GetMuzzleVelocity Weapon) 0.2))
      (Variables|/Game/TrueFPS/Items/Weapons/BP_WeaponMaster.BP_WeaponMaster_C|SetDamage Weapon (* (Variables|/Game/TrueFPS/Items/Weapons/BP_WeaponMaster.BP_WeaponMaster_C|GetDamage Weapon) 0.8))
      (Variables|/Game/TrueFPS/Items/Weapons/BP_WeaponMaster.BP_WeaponMaster_C|SetHearingRange Weapon (* (Variables|/Game/TrueFPS/Items/Weapons/BP_WeaponMaster.BP_WeaponMaster_C|GetHearingRange Weapon) 0.6)))))

(event EventRemoveAttachment
  (params (Weapon :type BP%20Weapon%20Master%20Object%20Reference))
  (|CallParentFunction Weapon)
  (Networking|SwitchHasAuthority
    (:Authority
      (Variables|/Game/TrueFPS/Items/Weapons/BP_WeaponMaster.BP_WeaponMaster_C|SetMuzzleVelocity Weapon (/ (Variables|/Game/TrueFPS/Items/Weapons/BP_WeaponMaster.BP_WeaponMaster_C|GetMuzzleVelocity Weapon) 0.2))
      (Variables|/Game/TrueFPS/Items/Weapons/BP_WeaponMaster.BP_WeaponMaster_C|SetDamage Weapon (/ (Variables|/Game/TrueFPS/Items/Weapons/BP_WeaponMaster.BP_WeaponMaster_C|GetDamage Weapon) 0.8))
      (Variables|/Game/TrueFPS/Items/Weapons/BP_WeaponMaster.BP_WeaponMaster_C|SetShotAudio Weapon (.ShotAudio (Utilities|GetClassDefaults (Utilities|GetClass Weapon))))
      (Variables|/Game/TrueFPS/Items/Weapons/BP_WeaponMaster.BP_WeaponMaster_C|SetHearingRange Weapon (/ (Variables|/Game/TrueFPS/Items/Weapons/BP_WeaponMaster.BP_WeaponMaster_C|GetHearingRange Weapon) 0.6)))))

(fn ConstructionScript
  (|CallParentFunction))