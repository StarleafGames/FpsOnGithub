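; BP_ShotRound is a shotgun-style ammo projectile that turns one fired round into a spread of pellets.
; On BeginPlay with authority, the original round spawns copies of its own class with randomized rotation within the spread, then destroys itself.
; Each pellet inherits velocity, damage, penetration, character and weapon, and is flagged non-original to prevent further splitting.
; Only these pellets run the parent round's Tick logic.
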(event EventBeginPlay
  (bind _returnvalue (Transformation|GetActorTransform))
  (bind _character (Variables|Default|GetCharacter))
  (bind _spread (Variables|Default|GetSpread))
  (bind _returnvalue_2 (* _spread -1.0))
  (Networking|SwitchHasAuthority
    (:Authority
      (if (Variables|Default|GetOriginal?)
        (for _index (range 1 (Variables|Default|GetPellets))
          (Game|SpawnActorfromClass (Utilities|GetClass self) (Math|Transform|MakeTransform (.location _returnvalue) (Math|Rotator|CombineRotators (.rotation _returnvalue) (Math|Rotator|MakeRotator (Math|Random|RandomFloatinRange _returnvalue_2 _spread) (Math|Random|RandomFloatinRange _returnvalue_2 _spread) (Math|Random|RandomFloatinRange _returnvalue_2 _spread))) (.scale _returnvalue)) "Undefined" 0 false (Variables|Default|GetMuzzleVelocity) (Variables|Default|GetDamage) (Variables|Default|GetPenetrationDistance) _character false (Variables|Default|GetWeapon) _character))
        (Actor|DestroyActor)
        (else
          (|CallParentFunction))))))

(event EventTick
  (params (DeltaSeconds :type Float%20%28single-precision%29))
  (if (not (Variables|Default|GetIsOriginal))
    (|CallParentFunction DeltaSeconds)))

(fn ConstructionScript
  (|CallParentFunction))