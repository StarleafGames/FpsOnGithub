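; BP_Grenade is a grenade actor for the TrueFPS game whose Explode event handles the blast and then destroys it.
; Explode plays sound, particle and camera shake effects and applies radial damage with falloff.
; A valid Character is credited as damage instigator and also triggers a "Hearing" noise event.
; A zero-length delay follows damage before the RadialForce impulse fires, presumably so physics reacts to damage results.
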(event EventBeginPlay
  (|CallParentFunction) ; This node is disabled and will not be called.\nDrag off pins to build functionality.
)

(event Collision|EventActorBeginOverlap
  (params (OtherActor :type Actor%20Object%20Reference)))

(event EventTick
  (params (DeltaSeconds :type Float%20%28single-precision%29)))

(event EventExplode
  (bind _returnvalue (Transformation|GetActorLocation))
  (Audio|PlaySoundatLocation "/Game/TrueFPS/Sounds/Sounds/UI/SCue_Grenade.SCue_Grenade" _returnvalue "0, 0, 0" 1.0 1.0 0.0 0 0 0 0)
  (Camera|PlayWorldCameraShake "/Game/TrueFPS/Items/Grenades/BP_Shake.BP_Shake_C" _returnvalue 1e+02 1.5e+03)
  (Effects|SpawnEmitteratLocation "/Game/TrueFPS/Effects/Effects/ParticleSystems/Weapons/RocketLauncher/Impact/P_Launcher_IH.P_Launcher_IH" _returnvalue)
  (Utilities|IsValid (Variables|Default|GetCharacter)
    (:Is%20Valid
      (Class|GameplayStatics|ApplyRadialDamagewithFalloff 1e+02 0.0 (Transformation|GetActorLocation) 2e+02 5e+02 1.0 0 0 self (Pawn|GetController (Variables|Default|GetCharacter)) "ECC_Visibility")
      (Class|AISenseHearing|ReportNoiseEvent (Transformation|GetActorLocation) 1.0 (Variables|Default|GetCharacter) 2e+03 "Hearing"))
    (:Is%20Not%20Valid
      (Class|GameplayStatics|ApplyRadialDamagewithFalloff 1e+02 0.0 (Transformation|GetActorLocation) 2e+02 5e+02 1.0 0 0 self 0 "ECC_Visibility")))
  (Utilities|FlowControl|Delay 0.0)
  (Class|RadialForceComponent|FireImpulse (Variables|Default|GetRadialForce))
  (Actor|DestroyActor))

(fn ConstructionScript
  (|CallParentFunction))