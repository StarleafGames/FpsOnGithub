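; Base Blueprint for TrueFPS grenade items, handling pin pull, cooking and throwing, with Explode left empty for child classes.
; Using it plays pin and looping hold montages while a server timeline updates the fuse Time, auto-throwing when finished.
; Throwing spawns the same class as a projectile carrying that Time, decrements the count and re-equips the previous weapon.
; The spawned projectile activates its movement and calls Explode after that delay, on authority only.
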(event Custom|Explode
  ;[0 0 0] Funtion For Child Classes
)

(event Custom|Throw
  (params (Character :type BP%20Character%20Master%20Object%20Reference))
  ;[0 0 0] Throw
  (Networking|SwitchHasAuthority
    (:Authority
      (if (> (Variables|Default|GetGrenadeCount) 0)
        (Game|SpawnActorfromClass (Utilities|GetClass self) (Math|Transform|MakeTransform (Transformation|GetActorLocation) (Pawn|GetControlRotation Character :!class /Script/Engine.Pawn) "1.000000,1.000000,1.000000") "Undefined" 0 true (Variables|Default|GetTime) Character 0)
        (Variables|Default|SetGrenadeCount (- (Variables|Default|GetGrenadeCount) 1))))))

(event Custom|MC%20Throw
  (params (Character :type BP%20Character%20Master%20Object%20Reference))
  ;[0 0 0] Throw
  (Animation|Montage|PlayMontage (Variables|/Script/Engine.Character|GetMesh Character) (Variables|Default|GetThrow%20Montage)
    (:then
      ;[0 0 0] Hold Grenade
      (bind _time (Timeline|Timer Stop)
        (:Update
          (Variables|Default|SetTime (* _time (Utilities|GetClassDefaults "BP_GrenadeMaster_C"))))
        (:Finished
          (if (not (Variables|Default|GetbHidden))
            (CallFunction|Throw (stale Custom|MC%20Grenade Character))
            (Default|SvrEquipItem (stale Custom|MC%20Grenade Character) (select (Variables|/Game/TrueFPS/Characters/BP_CharacterMaster.BP_CharacterMaster_C|GetWasUsingPrimary? (stale Custom|MC%20Grenade Character)) (Variables|/Game/TrueFPS/Characters/BP_CharacterMaster.BP_CharacterMaster_C|GetPrimary (stale Custom|MC%20Grenade Character)) (Variables|/Game/TrueFPS/Characters/BP_CharacterMaster.BP_CharacterMaster_C|GetSecondary (stale Custom|MC%20Grenade Character))) false false 1.0 false)
            (Utilities|FlowControl|Delay 0.1)
            (Variables|/Game/TrueFPS/Characters/BP_CharacterMaster.BP_CharacterMaster_C|SetIsUsing? (stale Custom|MC%20Grenade Character) false)))))
    (:OnBlendOut
      (Variables|/Game/TrueFPS/Characters/BP_CharacterMaster.BP_CharacterMaster_C|SetIsBusy? Character true)
      (Networking|SwitchHasAuthority
        (:Authority
          (CallFunction|Throw Character)
          (Utilities|IsValid Character
            (:Is%20Valid
              (Default|SvrEquipItem (stale EventStopUsing Character) (select (Variables|/Game/TrueFPS/Characters/BP_CharacterMaster.BP_CharacterMaster_C|GetWasUsingPrimary? Character) (Variables|/Game/TrueFPS/Characters/BP_CharacterMaster.BP_CharacterMaster_C|GetPrimary Character) (Variables|/Game/TrueFPS/Characters/BP_CharacterMaster.BP_CharacterMaster_C|GetSecondary Character)) false false 1.0 false))))))))

(event Custom|MC%20Grenade
  (params (Character :type BP%20Character%20Master%20Object%20Reference))
  (bind _mesh (Variables|/Script/Engine.Character|GetMesh Character))
  ;[0 0 0] Hold Grenade
  (Animation|Montage|PlayMontage _mesh (Variables|Default|GetRemove%20Pin%20Montage)
    (:OnBlendOut
      (Utilities|FlowControl|Sequence
        (:then_0
          (Animation|Montage|PlayMontage _mesh (Variables|Default|GetLoop%20Montage) :!label _label
            (:OnBlendOut
              (goto _label))))
        (:then_1
          (Networking|SwitchHasAuthority
            (:Authority
              (bind _time (Timeline|Timer PlayFromStart)
                (:Update
                  (Variables|Default|SetTime (* _time (Utilities|GetClassDefaults "BP_GrenadeMaster_C"))))
                (:Finished
                  (if (not (Variables|Default|GetbHidden))
                    (CallFunction|Throw Character)
                    (Default|SvrEquipItem Character (select (Variables|/Game/TrueFPS/Characters/BP_CharacterMaster.BP_CharacterMaster_C|GetWasUsingPrimary? Character) (Variables|/Game/TrueFPS/Characters/BP_CharacterMaster.BP_CharacterMaster_C|GetPrimary Character) (Variables|/Game/TrueFPS/Characters/BP_CharacterMaster.BP_CharacterMaster_C|GetSecondary Character)) false false 1.0 false)
                    (Utilities|FlowControl|Delay 0.1)
                    (Variables|/Game/TrueFPS/Characters/BP_CharacterMaster.BP_CharacterMaster_C|SetIsUsing? Character false)))))))))))

(event EventBeginPlay
  (|CallParentFunction)
  (Networking|SwitchHasAuthority
    (:Authority
      (if (Variables|Default|GetProjectile)
        (Components|Activation|Activate (Variables|Default|GetProjectileMovement) false)
        (Utilities|FlowControl|Delay (Variables|Default|GetTime))
        (CallFunction|Explode)))))

(event EventStartUsing
  (params (Character :type BP%20Character%20Master%20Object%20Reference) (Transform :type Transform))
  ;[0 0 0] Start Using
  (if (> (Variables|Default|GetGrenadeCount) 0)
    (Variables|Default|SetTime (Utilities|GetClassDefaults "BP_GrenadeMaster_C"))
    (Components|Timeline|SetPlayRate (Variables|Default|GetTimer) (/ 1.0 (Variables|Default|GetTime)))
    (Utilities|IsValid Character
      (:Is%20Valid
        (if (not (Variables|/Game/TrueFPS/Characters/BP_CharacterMaster.BP_CharacterMaster_C|GetIsUsing? Character))
          (Variables|/Game/TrueFPS/Characters/BP_CharacterMaster.BP_CharacterMaster_C|SetIsUsing? Character true)
          (CallFunction|MCGrenade Character))))))

(event EventStopUsing
  (params (Character :type BP%20Character%20Master%20Object%20Reference))
  ;[0 0 0] Throw
  (if (> (Variables|Default|GetGrenadeCount) 0)
    (Utilities|IsValid Character
      (:Is%20Valid
        (if (> (Variables|Default|GetGrenadeCount) 0)
          (CallFunction|MCThrow Character)
          (else
            (Default|SvrEquipItem Character (select (Variables|/Game/TrueFPS/Characters/BP_CharacterMaster.BP_CharacterMaster_C|GetWasUsingPrimary? (stale Custom|MC%20Throw Character)) (Variables|/Game/TrueFPS/Characters/BP_CharacterMaster.BP_CharacterMaster_C|GetPrimary (stale Custom|MC%20Throw Character)) (Variables|/Game/TrueFPS/Characters/BP_CharacterMaster.BP_CharacterMaster_C|GetSecondary (stale Custom|MC%20Throw Character))) false false 1.0 false)))))))

(fn ConstructionScript
  (|CallParentFunction))