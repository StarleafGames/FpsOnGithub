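; Master Blueprint for TrueFPS sniper weapons, implementing the reload sequence.
; ReloadStart checks character state, magazine space and reserve bullets, then MCReload plays long (empty) or short montages on the gun and character.
; On completion, the authority moves bullets from the reserve into the magazine, allowing an extra chambered round on short reloads.
; The reloading flag clears on completion or interruption, and blend-out triggers ClientBump.
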(event Custom|MC%20Reload
  (params (Long? :type Boolean) (Target :type BP%20Character%20Master%20Object%20Reference))
  (bind (_bulletref _bulletindex) (CallFunction|ReftoBullet))
  ;[0 0 0] Reload
  (Variables|Default|SetCharacter Target)
  (Variables|/Game/TrueFPS/Characters/BP_CharacterMaster.BP_CharacterMaster_C|SetIsReloading? Target true)
  (Animation|Montage|PlayMontage (Variables|Default|GetSkeletalMesh) (select Long? (Variables|Default|GetReloadLongMontageGun) (Variables|Default|GetReloadShortMontageGun))
    (:then
      (Animation|Montage|PlayMontage (Variables|/Script/Engine.Character|GetMesh (Variables|Default|GetCharacter)) (select Long? (Variables|Default|GetReloadLongMontage) (Variables|Default|GetReloadShortMontage))
        (:OnCompleted
          (Variables|/Game/TrueFPS/Characters/BP_CharacterMaster.BP_CharacterMaster_C|SetIsReloading? (Variables|Default|GetCharacter) false)
          (Networking|SwitchHasAuthority
            (:Authority
              (if Long?
                (Variables|Default|SetDifference (- (Variables|Default|GetMagSize) (Variables|Default|GetAmmoMag)))
                (if (>= (.amount _bulletref) (Variables|Default|GetDifference))
                  (Variables|Default|SetAmmoMag (+ (Variables|Default|GetAmmoMag) (Variables|Default|GetDifference)) :!label _label)
                  (CallFunction|SetBullet _bulletindex (- (.amount _bulletref) (Variables|Default|GetDifference)))
                  (else
                    (Variables|Default|SetAmmoMag (+ (Variables|Default|GetAmmoMag) (.amount _bulletref)) :!label _label_2)
                    (CallFunction|SetBullet _bulletindex)))
                (else
                  (Variables|Default|SetDifference (- (Variables|Default|GetMagSize) (- (Variables|Default|GetAmmoMag) 1)))
                  (if (>= (.amount _bulletref) (Variables|Default|GetDifference))
                    (goto _label)
                    (else
                      (goto _label_2)))))
              (Variables|Default|SetAmmoBag (- (Variables|Default|GetAmmoBag) (Variables|Default|GetDifference))))))
        (:OnBlendOut
          (CallFunction|ClientBump (Variables|Default|GetCharacter)))
        (:OnInterrupted
          (Variables|/Game/TrueFPS/Characters/BP_CharacterMaster.BP_CharacterMaster_C|SetIsReloading? (Variables|Default|GetCharacter) false))))))

(event EventReloadStart
  (params (Character :type BP%20Character%20Master%20Object%20Reference))
  ;[0 0 0] Reload
  (Variables|Default|SetCharacter Character)
  (if (not (or (Variables|/Game/TrueFPS/Characters/BP_CharacterMaster.BP_CharacterMaster_C|GetIsBusy? (Variables|Default|GetCharacter)) (Variables|/Game/TrueFPS/Characters/BP_CharacterMaster.BP_CharacterMaster_C|GetIsReloading? (Variables|Default|GetCharacter))))
    (if (not (== (Variables|Default|GetAmmoMag) (+ (Variables|Default|GetMagSize) 1)))
      (if (> (.amount (.BulletRef (CallFunction|ReftoBullet))) 0)
        (CallFunction|MCReload (== (Variables|Default|GetAmmoMag) 0) (Variables|Default|GetCharacter))))))

(fn ConstructionScript
  (|CallParentFunction))