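; Base shotgun Blueprint that overrides reloading to load one shell at a time.
; ReloadStart checks busy state, magazine space and reserve ammo, then MCReloadStart plays paired gun and character montages for start, loop and end.
; Each loop blend-out adds a shell on authority, deducting reserve ammo except for bots, and repeats until the magazine is full or reserve runs out.
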(event Custom|MC%20ReloadStart
  (params (Character :type BP%20Character%20Master%20Object%20Reference))
  (bind (_bulletref _bulletindex) (CallFunction|ReftoBullet))
  ;[0 0 0] Reload
  (bind _output_get (Variables|Default|SetCharacter Character))
  (Variables|/Game/TrueFPS/Characters/BP_CharacterMaster.BP_CharacterMaster_C|SetIsReloading? _output_get true)
  (Animation|Montage|PlayMontage (Variables|Default|GetSkeletalMesh) (Variables|Default|GetReloadStartGun)
    (:then
      (Animation|Montage|PlayMontage (Variables|/Script/Engine.Character|GetMesh _output_get) (Variables|Default|GetReloadStart)
        (:OnBlendOut
          (Animation|Montage|PlayMontage (Variables|Default|GetSkeletalMesh) (Variables|Default|GetReloadLoopGun) :!label _label
            (:then
              (Animation|Montage|PlayMontage (Variables|/Script/Engine.Character|GetMesh _output_get) (Variables|Default|GetReloadLoop)
                (:OnBlendOut
                  (if (> (.amount _bulletref) 0)
                    (Networking|SwitchHasAuthority
                      (:Authority
                        (Variables|Default|SetAmmoMag (+ (Variables|Default|GetAmmoMag) 1))
                        (if (not (Pawn|IsBotControlled _output_get))
                          (CallFunction|SetBullet _bulletindex (- (.amount _bulletref) 1))))
                      (:Remote
                        _))
                    (if (>= (Variables|Default|GetAmmoMag) (Variables|Default|GetMagSize))
                      _
                      (else
                        (goto _label))))
                  (Animation|Montage|PlayMontage (Variables|Default|GetSkeletalMesh) (Variables|Default|GetReloadEndGun)
                    (:then
                      (Animation|Montage|PlayMontage (Variables|/Script/Engine.Character|GetMesh _output_get) (Variables|Default|GetReloadEnd)
                        (:then
                          (Variables|/Game/TrueFPS/Characters/BP_CharacterMaster.BP_CharacterMaster_C|SetIsReloading? _output_get false)
                          (Variables|Default|SetDelayFinished true))))))))))))))

(event EventReloadStart
  (params (Character :type BP%20Character%20Master%20Object%20Reference))
  ;[0 0 0] Reload
  (Variables|Default|SetCharacter Character)
  (if (not (or (Variables|/Game/TrueFPS/Characters/BP_CharacterMaster.BP_CharacterMaster_C|GetIsBusy? (Variables|Default|GetCharacter)) (Variables|/Game/TrueFPS/Characters/BP_CharacterMaster.BP_CharacterMaster_C|GetIsReloading? (Variables|Default|GetCharacter))))
    (if (not (>= (Variables|Default|GetAmmoMag) (Variables|Default|GetMagSize)))
      (if (> (.amount (.BulletRef (CallFunction|ReftoBullet))) 0)
        (CallFunction|MCReloadStart (Variables|Default|GetCharacter))))))

(fn ConstructionScript
  (|CallParentFunction))