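; Behavior tree task that makes an AI character use its active item, such as firing a weapon, against the blackboard Target.
; A delayed loop re-triggers StartUsing so the AI can fire and reload, ending when the target character dies and clearing TargetAquired.
; The task never finishes execution itself.
; On abort, it clears controller focus, stops using the item and finishes the abort.
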(event EventReceiveExecuteAI
  (params (OwnerController :type AI%20Controller%20Object%20Reference) (ControlledPawn :type Pawn%20Object%20Reference))
  (bind _asbp_character_master (Utilities|Casting|CastToBP_CharacterMaster ControlledPawn))
  ;[0 0 0] Loop So AI Can Fire And Reload
  (Default|StartUsing _asbp_character_master (Variables|/Game/TrueFPS/Characters/BP_CharacterMaster.BP_CharacterMaster_C|GetActiveItem _asbp_character_master) :!label _label)
  (Utilities|FlowControl|Delay 0.5)
  (bind _asbp_character_master_2 (Utilities|Casting|CastToBP_CharacterMaster (AI|BehaviorTree|GetBlackboardValueasActor (Variables|Default|GetTarget)))
    (:then
      (if (not (Variables|/Game/TrueFPS/Characters/BP_CharacterMaster.BP_CharacterMaster_C|GetDead? _asbp_character_master_2))
        (goto _label)
        (else
          (Class|BTFunctionLibrary|SetBlackboardValueasBool (Variables|Default|GetTargetAquired) false))))
    (:CastFailed
      (goto _label))))

(event EventReceiveAbortAI
  (params (OwnerController :type AI%20Controller%20Object%20Reference) (ControlledPawn :type Pawn%20Object%20Reference))
  ;[0 0 0] Clear Focus And Stop Using
  (AI|ClearFocus OwnerController)
  (bind _asbp_character_master (Utilities|Casting|CastToBP_CharacterMaster ControlledPawn))
  (Default|StopUsing _asbp_character_master (Variables|/Game/TrueFPS/Characters/BP_CharacterMaster.BP_CharacterMaster_C|GetActiveItem _asbp_character_master))
  (Class|BTTaskBlueprintBase|FinishAbort))