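; Behavior tree task that advances an AI pawn's patrol point index stored in the blackboard.
; It casts the controlled pawn to BP_AIMaster and increments the index key, wrapping to 0 when the next index falls outside that pawn's PatrolPath.
; It finishes successfully after updating, or fails if the pawn is not a BP_AIMaster.
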(event EventReceiveExecuteAI
  (params (OwnerController :type AI%20Controller%20Object%20Reference) (ControlledPawn :type Pawn%20Object%20Reference))
  (bind _bppathindex (Variables|Default|GetBPPathIndex))
  (bind _returnvalue (Class|BTFunctionLibrary|GetBlackboardValueasInt _bppathindex))
  (bind _returnvalue_2 (+ _returnvalue 1))
  (bind _asbp_aimaster (Utilities|Casting|CastToBP_AIMaster ControlledPawn)
    (:then
      ;[0 0 0] Loop Back To Start If Index Isnt Valid (End Of Path)
      (if (not (Utilities|Array|IsValidIndex (Variables|/Game/TrueFPS/Characters/AI/BP_AIMaster.BP_AIMaster_C|GetPatrolPath _asbp_aimaster) _returnvalue_2))
        (Class|BTFunctionLibrary|SetBlackboardValueasInt (Variables|Default|GetBPPathIndex))
        (else
          (Class|BTFunctionLibrary|SetBlackboardValueasInt (Variables|Default|GetBPPathIndex) _returnvalue_2)))
      (AI|BehaviorTree|FinishExecute true))
    (:CastFailed
      (AI|BehaviorTree|FinishExecute false))))