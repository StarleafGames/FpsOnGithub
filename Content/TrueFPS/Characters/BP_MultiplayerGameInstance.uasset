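; Multiplayer game instance for TrueFPS that hosts and joins online sessions for the first local player controller.
; CreateGame hosts a two-connection online session and opens the default 1v1 map as a listen server.
; HOSTSESSION does the same with caller-supplied connections, LAN flag and level name, printing success or failure.
; JoinGame joins a passed-in search result with no success or failure handling.
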(event Custom|HOST%20SESSION
  (params (PublicConnections :type Integer) (bUseLAN :type Boolean) (LevelName :type Name))
  (|Session (Game|GetPlayerController 0) PublicConnections bUseLAN
    (:OnSuccess
      (Development|PrintString "Successfully created a session")
      (Game|OpenLevel(byName) LevelName true "listen"))
    (:OnFailure
      (Development|PrintString "Failed to created a session"))))

(event Custom|Create%20Game
  (|Session (Game|GetPlayerController 0) 2 false
    (:OnSuccess
      (Game|OpenLevel(byObjectReference) "/Game/TrueFPS/Maps/Default_1v1_Map.Default_1v1_Map" true "listen"))))

(event Custom|Join%20Game
  (params (SearchResult :type Blueprint%20Session%20Result%20Structure%20%28by%20ref%29))
  (|JoinSession (Game|GetPlayerController 0) SearchResult))