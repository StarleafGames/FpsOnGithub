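; Deathmatch player character Blueprint that tints its body mesh with a replicated team color.
; When TeamColor_0 replicates, its OnRep creates a dynamic instance of M_UE4Man_Body, sets the BodyColor parameter and applies it to mesh material slot 0.
; The event graph holds only disabled placeholder events, and the construction script just calls its parent.
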(event EventBeginPlay
  (|CallParentFunction))

(event Collision|EventActorBeginOverlap
  (params (OtherActor :type Actor%20Object%20Reference)))

(event EventTick
  (params (DeltaSeconds :type Float%20%28single-precision%29))
  (|CallParentFunction DeltaSeconds) ; This node is disabled and will not be called.\nDrag off pins to build functionality.
)

(fn ConstructionScript
  (|CallParentFunction))

(fn OnRepTeamColor0
  (bind _returnvalue (Rendering|Material|CreateDynamicMaterialInstance "/Game/TrueFPS/Characters/Animations/UE4_Mannequin/Materials/M_UE4Man_Body.M_UE4Man_Body" "None" "None" :!class /Script/Engine.KismetMaterialLibrary))
  (Rendering|Material|SetVectorParameterValue _returnvalue "BodyColor" (Variables|Default|GetTeamColor_0) :!class /Script/Engine.MaterialInstanceDynamic)
  (Rendering|Material|SetMaterial (Variables|Character|GetMesh) 0 _returnvalue))